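; Automatic elevator actor that cycles down and up through a set number of levels without player input, starting on BeginPlay.
; Down and Up timelines each move it one level by adding a vector track to a stored base location, updated after each leg.
; A level counter, seeded from NumBelow, reverses direction when it reaches NumLevels, with a short pause after every stop.
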(event `self.ReceiveBeginPlay`
  ;[1 1 1] Init
  (set `self.InitLocal` (`self.K2_GetActorLocation`))
  (`KismetSystemLibrary.Delay` 2.0)
  (set `self.level` (`self.numBelow`))
  ;[1 1 1] GoingDown
  (bind (_direction _newtrack_0) (`Timeline|DownTimeline` :!via `PlayFromStart` :!label _label)
    (:`Update`
      (bind _returnvalue (+ _newtrack_0 (`self.InitLocal`)))
      (`self.K2_SetActorLocation` _returnvalue))
    (:`Finished`
      (set `self.InitLocal` _returnvalue)
      (`KismetSystemLibrary.Delay` 2.0)
      (bind _output_get (set `self.level` (+ (`self.level`) 1)))
      (if (< _output_get (`self.numLevels`))
        (goto _label :!via `PlayFromStart`)
        (else
          (set `self.level` 0)
          ;[1 1 1] GoingUp
          (bind (_direction_2 _newtrack_0_2) (`Timeline|UpTimeline` :!via `PlayFromStart` :!label _label_2)
            (:`Update`
              (bind _returnvalue_2 (+ _newtrack_0_2 (`self.InitLocal`)))
              (`self.K2_SetActorLocation` _returnvalue_2))
            (:`Finished`
              (set `self.InitLocal` _returnvalue_2)
              (`KismetSystemLibrary.Delay` 2.0)
              (bind _output_get_2 (set `self.level` (+ (`self.level`) 1)))
              (if (< _output_get_2 (`self.numLevels`))
                (goto _label_2 :!via `PlayFromStart`)
                (else
                  (set `self.level` 0)
                  (goto _label :!via `PlayFromStart`))))))))))

(fn `UserConstructionScript`)