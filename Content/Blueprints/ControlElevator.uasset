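; Player-operated elevator actor that moves up and down between levels with the W and S keys.
; Overlapping the actor enables player 0's input on it, and leaving disables it.
; Each press plays a GoUp or GoDown timeline that offsets the actor from its last stop.
; A Moving flag blocks presses mid-travel, and LevelOn is bounded between zero and NumLevels.
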(event `self.ReceiveBeginPlay`
  (set `self.InitLocal` (`self.K2_GetActorLocation`)))

(event `Key|W`
  (params (Key :type "Key Structure"))
  (:`Pressed`
    (if (`self.moving`)
      _
      (elif (< (`self.levelOn`) (`self.numLevels`))
        (set `self.moving` true)
        (bind (_direction _newtrack_0) (`Timeline|GoUp` :!via `PlayFromStart`)
          (:`Update`
            (bind _returnvalue (+ _newtrack_0 (`self.InitLocal`)))
            (`self.K2_SetActorLocation` _returnvalue))
          (:`Finished`
            (set `self.InitLocal` _returnvalue)
            (set `self.levelOn` (+ (`self.levelOn`) 1))
            (set `self.moving` false)))))))

(event `self.ReceiveActorBeginOverlap`
  (params (OtherActor :type "Actor Object Reference"))
  (`self.EnableInput` (`GameplayStatics.GetPlayerController` 0))
  (`KismetSystemLibrary.PrintString` "Enter"))

(event `self.ReceiveActorEndOverlap`
  (params (OtherActor :type "Actor Object Reference"))
  (`self.DisableInput` (`GameplayStatics.GetPlayerController` 0))
  (`KismetSystemLibrary.PrintString` "Exit"))

(event `Key|S`
  (params (Key :type "Key Structure"))
  (:`Pressed`
    (if (`self.moving`)
      _
      (elif (> (`self.levelOn`) 0)
        (set `self.moving` true)
        (bind (_direction _newtrack_0) (`Timeline|GoDown` :!via `PlayFromStart`)
          (:`Update`
            (bind _returnvalue (+ _newtrack_0 (`self.InitLocal`)))
            (`self.K2_SetActorLocation` _returnvalue))
          (:`Finished`
            (set `self.InitLocal` _returnvalue)
            (set `self.levelOn` (- (`self.levelOn`) 1))
            (set `self.moving` false)))))))

(fn `UserConstructionScript`)