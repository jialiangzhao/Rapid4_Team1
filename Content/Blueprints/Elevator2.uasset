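; Elevator actor that cycles up and down between floors on its own, or is driven by the player while they stand in it.
; Automatic mode steps one fixed-height level at a time with a delay between stops, reversing at the top and bottom.
; Overlap by BP_ThirdPersonCharacter sets Controlling and enables W/S input for single-level moves; leaving resumes automatic mode.
; Timelines lerp the root's relative location, with a Moving flag blocking overlapping moves.
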(event `playAutomatic`
  ;[1 1 1] Automatic Movement
  (`KismetSystemLibrary.Delay` (`self.delayAmount`))
  (if (`self.controlling`)
    _
    (elif (< (`self.levelOn`) (`self.numLevels`))
      (if (`self.moving`) :!label _label
        _
        (elif (not (`self.controlling`))
          (set `self.moving` true)
          (bind _output_get (set `self.endLocation` (+ (`self.endLocation`) (0.0 0.0 500.0))))
          (bind (_direction _newtrack_0) (`Timeline|autoUp` :!via `PlayFromStart`)
            (:`Update`
              (`SceneComponent.K2_SetRelativeLocation` (`self.DefaultSceneRoot`) (`KismetMathLibrary.VLerp` (`self.startLocation`) _output_get _newtrack_0) false false))
            (:`Finished`
              (set `self.startLocation` _output_get)
              (set `self.levelOn` (+ (`self.levelOn`) 1))
              (`KismetSystemLibrary.Delay` (`self.delayAmount`))
              (set `self.moving` false)
              (if (`self.controlling`)
                _
                (elif (< (`self.levelOn`) (`self.numLevels`))
                  (goto _label)
                  (else
                    (if (`self.moving`) :!label _label_2
                      _
                      (elif (not (`self.controlling`))
                        (set `self.moving` true)
                        (bind _output_get_2 (set `self.endLocation` (+ (`self.endLocation`) (0.0 0.0 -500.0))))
                        (bind (_direction_2 _newtrack_0_2) (`Timeline|autoDown` :!via `PlayFromStart`)
                          (:`Update`
                            (`SceneComponent.K2_SetRelativeLocation` (`self.DefaultSceneRoot`) (`KismetMathLibrary.VLerp` (`self.startLocation`) _output_get_2 _newtrack_0_2) false false))
                          (:`Finished`
                            (set `self.startLocation` _output_get_2)
                            (set `self.levelOn` (- (`self.levelOn`) 1))
                            (`KismetSystemLibrary.Delay` (`self.delayAmount`))
                            (set `self.moving` false)
                            (if (`self.controlling`)
                              _
                              (elif (> (`self.levelOn`) 1)
                                (goto _label_2)
                                (else
                                  (goto _label)))))))))))))))
      (else
        (goto _label_2)))))

(event `self.ReceiveBeginPlay`
  ;[1 1 1] Start
  (bind _output_get (set `self.startLocation` (`self.K2_GetActorLocation`)))
  (set `self.endLocation` _output_get)
  (if (not (`self.controlling`))
    (`self.playAutomatic`)))

(event `Key|W`
  (params (Key :type "Key Structure"))
  ;[1 1 1] Manual Movement
  (:`Pressed`
    (if (`self.moving`)
      _
      (elif (< (`self.levelOn`) (`self.numLevels`))
        (set `self.moving` true)
        (bind _output_get (set `self.endLocation` (+ (`self.endLocation`) (0.0 0.0 500.0))))
        (bind (_direction _newtrack_0) (`Timeline|manualUp` :!via `PlayFromStart`)
          (:`Update`
            (`SceneComponent.K2_SetRelativeLocation` (`self.DefaultSceneRoot`) (`KismetMathLibrary.VLerp` (`self.startLocation`) _output_get _newtrack_0) false false))
          (:`Finished`
            (set `self.startLocation` _output_get)
            (set `self.levelOn` (+ (`self.levelOn`) 1))
            (`KismetSystemLibrary.Delay` 0.2)
            (set `self.moving` false)))))))

(event `self.ReceiveActorBeginOverlap`
  (params (OtherActor :type "Actor Object Reference"))
  ;[1 1 1] Check Control
  (cast `/Game/ThirdPerson/Blueprints/BP_ThirdPersonCharacter` OtherActor)
  (set `self.controlling` true)
  (`self.EnableInput` (`GameplayStatics.GetPlayerController` 0)))

(event `self.ReceiveActorEndOverlap`
  (params (OtherActor :type "Actor Object Reference"))
  ;[1 1 1] Check Control
  (cast `/Game/ThirdPerson/Blueprints/BP_ThirdPersonCharacter` OtherActor)
  (set `self.controlling` false)
  (`self.DisableInput` (`GameplayStatics.GetPlayerController` 0))
  (`self.playAutomatic`))

(event `Key|S`
  (params (Key :type "Key Structure"))
  ;[1 1 1] Manual Movement
  (:`Pressed`
    (if (`self.moving`)
      _
      (elif (> (`self.levelOn`) 1)
        (set `self.moving` true)
        (bind _output_get (set `self.endLocation` (- (`self.endLocation`) (0.0 0.0 500.0))))
        (bind (_direction _newtrack_0) (`Timeline|Timeline_0` :!via `PlayFromStart`)
          (:`Update`
            (`SceneComponent.K2_SetRelativeLocation` (`self.DefaultSceneRoot`) (`KismetMathLibrary.VLerp` (`self.startLocation`) _output_get _newtrack_0) false false))
          (:`Finished`
            (set `self.startLocation` _output_get)
            (set `self.levelOn` (- (`self.levelOn`) 1))
            (`KismetSystemLibrary.Delay` 0.2)
            (set `self.moving` false)))))))

(fn `UserConstructionScript`)