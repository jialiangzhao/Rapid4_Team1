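; Saw trap actor that launches along Y from one of two fixed endpoints and damages the player on overlap while moving.
; Tick polls ShootSaw and, if the saw is idle, starts it from the endpoint farther from the player in Y.
; Two timelines supply offsets from those endpoints and clear IsMoving when finished.
; The right timeline uses Play, while the left uses PlayFromStart.
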(event `self.ReceiveActorBeginOverlap`
  (params (OtherActor :type "Actor Object Reference"))
  (bind _returnvalue (`GameplayStatics.GetPlayerCharacter` 0))
  ;[1 1 1] Check for collision
  (if (`self.isMoving`)
    (if (== OtherActor _returnvalue)
      (bind _asbp_third_person_character (cast `/Game/ThirdPerson/Blueprints/BP_ThirdPersonCharacter` _returnvalue))
      (`/Game/ThirdPerson/Blueprints/BP_ThirdPersonCharacter.getDamage` _asbp_third_person_character))))

(event `self.ReceiveBeginPlay`
  (bind (_returnvalue_x _returnvalue_y _returnvalue_z) (`KismetMathLibrary.BreakVector` (`self.K2_GetActorLocation`)))
  ;[1 1 1] Set Locations
  (set `self.leftLocation` (`KismetMathLibrary.MakeVector` _returnvalue_x 190.0 _returnvalue_z))
  (set `self.rightLocation` (`KismetMathLibrary.MakeVector` _returnvalue_x 3080.0 _returnvalue_z)))

(event `playSaw`
  (params (shootSaw :type Boolean))
  (bind _returnvalue (`self.K2_GetActorLocation` (`GameplayStatics.GetPlayerCharacter` 0)))
  (bind (_returnvalue_x _returnvalue_y) (`KismetMathLibrary.BreakVector` (- _returnvalue (`self.leftLocation`))))
  (bind (_returnvalue_x_2 _returnvalue_y_2) (`KismetMathLibrary.BreakVector` (- _returnvalue (`self.rightLocation`))))
  ;[1 1 1] Move Saw
  (if shootSaw
    (if (not (`self.isMoving`))
      (set `self.isMoving` true)
      (if (< (`KismetMathLibrary.Abs` _returnvalue_y) (`KismetMathLibrary.Abs` _returnvalue_y_2))
        (bind (_direction _newtrack_0) (`Timeline|rightMoveSaw`)
          (:`Update`
            (`self.K2_SetActorLocation` (+ (`self.rightLocation`) _newtrack_0)))
          (:`Finished`
            (set `self.isMoving` false)))
        (else
          (bind (_direction_2 _newtrack_0_2) (`Timeline|leftMoveSaw` :!via `PlayFromStart`)
            (:`Update`
              (`self.K2_SetActorLocation` (+ (`self.leftLocation`) _newtrack_0_2)))
            (:`Finished`
              (set `self.isMoving` false))))))))

(event `self.ReceiveTick`
  (params (DeltaSeconds :type "Float (single-precision)"))
  (`self.playSaw` (`self.shootSaw`)))

(fn `UserConstructionScript`)