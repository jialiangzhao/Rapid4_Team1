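; Elevator actor that shuttles between levels on its own and hands control to the player while they overlap it.
; Timelines add an offset to a stored base location, which updates along with the level counter after each one-level move.
; Automatic mode pauses briefly at each stop and reverses at the top and bottom.
; Overlap enables W/S input for single-level moves; leaving resumes automatic travel.
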(event `self.ReceiveBeginPlay`
  ;[1 1 1] Init
  (set `self.InitLocal` (`self.K2_GetActorLocation`))
  (set `self.level` (`self.numBelow`))
  (`KismetSystemLibrary.Delay` 2.0)
  (if (not (`self.controlling`))
    (`self.Play`)))

(event `Play`
  (if (< (`self.level`) (`self.numLevels`))
    (set `self.Moving` true :!label _label)
    ;[1 1 1] GoingUp
    (bind (_direction _newtrack_0) (`Timeline|UpTimeline` :!via `PlayFromStart`)
      (:`Update`
        (bind _returnvalue (+ _newtrack_0 (`self.InitLocal`)))
        (`self.K2_SetActorLocation` _returnvalue))
      (:`Finished`
        (set `self.InitLocal` _returnvalue)
        (bind _output_get (set `self.level` (+ (`self.level`) 1)))
        (set `self.Moving` false)
        (if (not (`self.controlling`))
          (`KismetSystemLibrary.Delay` 2.0)
          (if (< _output_get (`self.numLevels`))
            (goto _label)
            (else
              ;[1 1 1] GoingDown
              (set `self.Moving` true :!label _label_2)
              (bind (_direction_2 _newtrack_0_2) (`Timeline|DownTimeline` :!via `PlayFromStart`)
                (:`Update`
                  (bind _returnvalue_2 (+ _newtrack_0_2 (`self.InitLocal`)))
                  (`self.K2_SetActorLocation` _returnvalue_2))
                (:`Finished`
                  (set `self.InitLocal` _returnvalue_2)
                  (bind _output_get_2 (set `self.level` (- (`self.level`) 1)))
                  (set `self.Moving` false)
                  (if (not (`self.controlling`))
                    (`KismetSystemLibrary.Delay` 2.0)
                    (if (> _output_get_2 0)
                      (goto _label_2)
                      (else
                        (goto _label)))))))))))
    (else
      (goto _label_2))))

(event `Key|W`
  (params (Key :type "Key Structure"))
  (:`Pressed`
    (if (`self.moving`)
      _
      (elif (< (`self.level`) (`self.numLevels`))
        (set `self.moving` true)
        (bind (_direction _newtrack_0) (`Timeline|Timeline_0` :!via `PlayFromStart`)
          (:`Update`
            (bind _returnvalue (+ _newtrack_0 (`self.InitLocal`)))
            (`self.K2_SetActorLocation` _returnvalue))
          (:`Finished`
            (set `self.InitLocal` _returnvalue)
            (set `self.level` (+ (`self.level`) 1))
            (set `self.moving` false)))))))

(event `self.ReceiveActorBeginOverlap`
  (params (OtherActor :type "Actor Object Reference"))
  (if (== OtherActor (`GameplayStatics.GetPlayerCharacter` 0))
    (`self.EnableInput` (`GameplayStatics.GetPlayerController` 0))
    (set `self.controlling` true)
    (`KismetSystemLibrary.PrintString` "Enter")))

(event `self.ReceiveActorEndOverlap`
  (params (OtherActor :type "Actor Object Reference"))
  (if (== OtherActor (`GameplayStatics.GetPlayerCharacter` 0))
    (`self.DisableInput` (`GameplayStatics.GetPlayerController` 0))
    (set `self.controlling` false)
    (`self.Play`)))

(event `Key|S`
  (params (Key :type "Key Structure"))
  (:`Pressed`
    (if (`self.moving`)
      _
      (elif (> (`self.level`) 0)
        (set `self.moving` true)
        (bind (_direction _newtrack_0) (`Timeline|Timeline_1` :!via `PlayFromStart`)
          (:`Update`
            (bind _returnvalue (+ _newtrack_0 (`self.InitLocal`)))
            (`self.K2_SetActorLocation` _returnvalue))
          (:`Finished`
            (set `self.InitLocal` _returnvalue)
            (set `self.level` (- (`self.level`) 1))
            (set `self.moving` false)))))))

(fn `UserConstructionScript`)